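; Base interactable door Blueprint that drives its rotation with tweens.
; On interaction, a valid open tween is flipped and replayed only if the door is flagged as opened.
; Without a valid tween, it calls a zero-duration rotate to zero rotation.
; The file never assigns the tween or the opened flag, and two audio SetSound nodes are left unconnected.
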(event OnInteract(InteractableComponent)
  (if (Utilities|IsValid (Variables|Default|GetDoorOpenTween))
    (if (Variables|InteractionInfo|GetIsDoorOpened)
      (bind _returnvalue (Class|Tween|Flip (Variables|Default|GetDoorOpenTween)))
      (Class|Tween|Play _returnvalue))
    (else
      (Class|TransformTweenFunctions|DoRotate 0 "0, 0, 0" 0.0))))

(event EventBeginPlay)

(fn ConstructionScript)
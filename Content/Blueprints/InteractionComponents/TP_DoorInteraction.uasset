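; Interaction component that swings a door mesh open and closed and plays the matching open or close sound.
; The first Interact creates a local-rotation tween of 90 degrees with configurable duration and easing.
; Auto-kill is disabled so later interactions flip and replay that same tween instead of creating a new one.
; Setup receives the mesh and audio source, adding an audio component to the owner if none is valid.
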(event EventBeginPlay
  (Variables|Default|SetFirstInteraction true))

(event EventInteract
  (if (Variables|Default|GetFirstInteraction)
    (Variables|Default|SetFirstInteraction false)
    (bind _returnvalue (Class|ShortcutExtensions|DoLocalRotateComponent (Variables|Default|GetDoorMesh) "0.000000,-90.000000,0.000000" (Variables|InteractionInfo|GetDuration)))
    (bind _output_get (Variables|Default|SetInteractionTween _returnvalue))
    (bind _returnvalue_2 (Class|Tween|SetAutoKill _output_get false))
    (Class|Tween|SetEaseType _returnvalue_2 (Variables|InteractionInfo|GetEaseType))
    (else
      (bind _returnvalue_3 (Class|Tween|Flip (Variables|Default|GetInteractionTween)))
      (Class|Tween|Play _returnvalue_3)))
  (CallFunction|PlayDoorOpenCloseSound)
  (Variables|InteractionInfo|SetIsDoorOpened (not (Variables|InteractionInfo|GetIsDoorOpened))))

(fn SetDoorMesh
  (params (DoorMesh :type Static%20Mesh%20Component%20Object%20Reference))
  (Variables|Default|SetDoorMesh DoorMesh))

(fn SetAudioSource
  (params (AudioSource :type Audio%20Component%20Object%20Reference))
  (Variables|Default|SetDoorAudioSource AudioSource))

(fn PlayDoorOpenCloseSound
  (bind _dooraudiosource (Variables|Default|GetDoorAudioSource))
  (if (Variables|InteractionInfo|GetIsDoorOpened)
    (Audio|Components|Audio|SetSound _dooraudiosource (Variables|CustomSounds|GetDoorCloseSound))
    (else
      (Audio|Components|Audio|SetSound _dooraudiosource (Variables|CustomSounds|GetDoorOpenSound))))
  (Audio|Components|Audio|Play _dooraudiosource 0.0))

(fn Setup
  (params (DoorMesh :type Static%20Mesh%20Component%20Object%20Reference) (AudioSource :type Audio%20Component%20Object%20Reference))
  (Variables|Default|SetDoorMesh DoorMesh)
  (bind _output_get (Variables|Default|SetDoorAudioSource AudioSource))
  (if (not (Utilities|IsValid _output_get))
    (bind _returnvalue (Game|AddComponentbyClass (Components|GetOwner) "/Script/Engine.AudioComponent" false))
    (Variables|Default|SetDoorAudioSource _returnvalue)))